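; Enemy archer AI that patrols and sends the player to LevelLoop with a defeat widget on overlap.
; Patrol repeats slow moves to random reachable nearby points while IsChasing is false.
; The first PawnSensing sighting starts a faster chase only if IsChasing is true, but this graph never sets it true and the DoOnce never resets.
; The timer for ResumePatrol is unwired.
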(event OnSeePawn(PawnSensing)
  (params (Pawn :type Pawn%20Object%20Reference))
  (Utilities|FlowControl|DoOnce false
    (:Completed
      (if (Variables|Default|GetIsChasing)
        (bind _asbp_third_person_character (Utilities|Casting|CastToBP_ThirdPersonCharacter Pawn))
        (Components|Movement|StopMovementImmediately (Variables|Character|GetCharacterMovement))
        (Variables|/Script/Engine.CharacterMovementComponent|SetMaxWalkSpeed (Variables|Character|GetCharacterMovement) 6e+02)
        (AI|AIMoveTo self "0, 0, 0" _asbp_third_person_character 1.2e+02 false)))))

(event Custom|Patrol
  (if (not (Variables|Default|GetIsChasing))
    (Variables|/Script/Engine.CharacterMovementComponent|SetMaxWalkSpeed (Variables|Character|GetCharacterMovement) 2.5e+02)
    (Components|Movement|StopMovementImmediately (Variables|Character|GetCharacterMovement))
    (AI|AIMoveTo self (.RandomLocation (AI|Navigation|GetRandomReachablePointinRadius (Transformation|GetActorLocation) 5e+02 0 0)) 0 8e+01 false
      (:OnSuccess
        (CallFunction|Patrol)))))

(event Custom|ResumePatrol
  (Variables|Default|SetIsChasing false)
  (CallFunction|Patrol))

(event EventBeginPlay
  (CallFunction|Patrol))

(event Collision|EventActorBeginOverlap
  (params (OtherActor :type Actor%20Object%20Reference))
  (Utilities|Casting|CastToBP_ThirdPersonCharacter OtherActor)
  (Game|OpenLevel(byName) "LevelLoop")
  (bind _returnvalue (UserInterface|CreateWidget "/Game/UI/W_Defeat.W_Defeat_C"))
  (UserInterface|Viewport|AddtoViewport _returnvalue 0)
  (Utilities|FlowControl|Delay 3.0)
  (Viewport|RemoveAllWidgets))

(fn ConstructionScript)