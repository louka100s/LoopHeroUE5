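; Board-game player pawn that moves along linked tiles, tracking resources and artifacts, with HUD, victory and defeat widgets.
; RollDice draws a 1–6 move count, charges resources, destroys the pawn on depletion, and calls Avancer both before and after that charge.
; Avancer hops through each tile's CaseSuivante on a delayed recursive loop, then DispatchVerifCase applies the landing tile's effect: artifact, resource change, or minigame level load.
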(event Custom|RollDice
  (Variables|Default|SetDeplacementsRestants (Math|Random|RandomIntegerinRange 1 6))
  (CallFunction|Avancer)
  (Variables|Default|SetRessources (- (Variables|Default|GetRessources) 5))
  (if (<= (Variables|Default|GetRessources) 0)
    (bind _returnvalue (UserInterface|CreateWidget "/Game/UI/W_Defeat.W_Defeat_C"))
    (UserInterface|Viewport|AddtoViewport _returnvalue 0)
    (Actor|DestroyActor)
    (else
      (CallFunction|Avancer))))

(event Custom|Avancer
  (if (> (Variables|Default|GetDeplacementsRestants) 0)
    (Utilities|FlowControl|Sequence
      (:then_0
        (Transformation|SetActorLocation (Math|Vector|MakeVector (.x (Transformation|GetActorLocation (Variables|/Game/Blueprint/BP_Case.BP_Case_C|GetCaseSuivante (Variables|Default|GetCaseActuelle)))) (.y (Transformation|GetActorLocation (Variables|/Game/Blueprint/BP_Case.BP_Case_C|GetCaseSuivante (Variables|Default|GetCaseActuelle)))) (+ (.z (Transformation|GetActorLocation (Variables|/Game/Blueprint/BP_Case.BP_Case_C|GetCaseSuivante (Variables|Default|GetCaseActuelle)))) 5e+01)) false false))
      (:then_1
        (Variables|Default|SetCaseActuelle (Variables|/Game/Blueprint/BP_Case.BP_Case_C|GetCaseSuivante (Variables|Default|GetCaseActuelle))))
      (:then_2
        (Variables|Default|SetDeplacementsRestants (- (Variables|Default|GetDeplacementsRestants) 1)))
      (:then_3
        (Utilities|FlowControl|Delay 0.5)
        (if (== (Variables|Default|GetDeplacementsRestants) 0)
          (CallFunction|DispatchVerifCase)
          (else
            (CallFunction|Avancer)))))))

(event Custom|DispatchVerifCase
  (switch string (Variables|/Game/Blueprint/BP_Case.BP_Case_C|GetTypeCase (Variables|Default|GetCaseActuelle))
    (:Artéfact
      (Variables|Default|SetArtéfacts (+ (Variables|Default|GetArtéfacts) 1))
      (if (>= (Variables|Default|GetArtéfacts) 2)
        (bind _returnvalue (UserInterface|CreateWidget "/Game/UI/W_Victory.W_Victory_C"))
        (UserInterface|Viewport|AddtoViewport _returnvalue 0)))
    (:Ruine
      (Variables|Default|SetRessources (+ (Variables|Default|GetRessources) 30)))
    (:Combat
      (Variables|Default|SetRessources (- (Variables|Default|GetRessources) 15)))
    (:Dialog
      (if (>= (Variables|/Game/Blueprint/BP_Case.BP_Case_C|GetVisitDialogCase (Variables|Default|GetCaseActuelle)) 1)
        (Game|OpenLevel(byName) "HideandSeek_Level")
        (else
          (Game|OpenLevel(byName) "MiniGame")
          (Variables|/Game/Blueprint/BP_Case.BP_Case_C|SetVisitDialogCase (Variables|Default|GetCaseActuelle) (+ (Variables|/Game/Blueprint/BP_Case.BP_Case_C|GetVisitDialogCase (Variables|Default|GetCaseActuelle)) 1)))))))

(event EventBeginPlay
  (bind _caseactuelle (Variables|Default|GetCaseActuelle))
  (bind _returnvalue (Transformation|GetActorLocation _caseactuelle))
  (Transformation|SetActorLocation (Math|Vector|MakeVector (.x _returnvalue) (.y _returnvalue) 0.0) false false)
  (bind _returnvalue_2 (UserInterface|CreateWidget "/Game/UI/W_Interface.W_Interface_C"))
  (UserInterface|Viewport|AddtoViewport _returnvalue_2 0)
  (Variables|/Script/Engine.PlayerController|SetbShowMouseCursor (Game|GetPlayerController 0) true))

(fn ConstructionScript)