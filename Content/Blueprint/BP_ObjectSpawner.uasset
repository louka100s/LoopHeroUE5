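; BP_ObjectSpawner spawns a BP_FallingObjects actor when play begins, always spawning regardless of collision.
; It starts a looping timer at SpawnInterval with no event shown bound, so the spawn follows directly and runs once.
; The spawn point is in world space at zero height, with X and Y random ranges using SpawnAreaSize as both bounds, so the position is effectively fixed.
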(event EventBeginPlay
  (Utilities|Time|SetTimerbyEvent "" (Variables|Default|GetSpawnInterval) true)
  (Game|SpawnActorfromClass "/Game/Blueprint/BP_FallingObjects.BP_FallingObjects_C" (Math|Conversions|ToTransform(Vector) (Math|Vector|MakeVector (Math|Random|RandomFloatinRange (Variables|Default|GetSpawnAreaSize) (Variables|Default|GetSpawnAreaSize)) (Math|Random|RandomFloatinRange (Variables|Default|GetSpawnAreaSize) (Variables|Default|GetSpawnAreaSize)) 0.0)) "AlwaysSpawn" "MultiplyWithRoot" 0 0))

(fn ConstructionScript)